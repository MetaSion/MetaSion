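; BP_CJS_TextActor is a test actor that shows a short sequence of three messages on a text render component.
; On BeginPlay it sets the first text input, then switches to the second and third with two-second delays between them.
; The messages come from three text variables, and the construction script is empty.
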(event EventBeginPlay
  (Rendering|Components|TextRender|SetText (Variables|Default|GetTextRender) (Variables|Default|GetTextInput_1))
  (Utilities|FlowControl|Delay 2.0)
  (Rendering|Components|TextRender|SetText (Variables|Default|GetTextRender) (Variables|Default|GetTextInput_2))
  (Utilities|FlowControl|Delay 2.0)
  (Rendering|Components|TextRender|SetText (Variables|Default|GetTextRender) (Variables|Default|GetTextInput_3)))

(fn ConstructionScript)