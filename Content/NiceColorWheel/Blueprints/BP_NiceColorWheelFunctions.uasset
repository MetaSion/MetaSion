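; Function library for the Nice Color Wheel widgets that combines wheel color with slider value and persists each control's HSV.
; All entries live in one delimited string on BP_NiceColorWheel_SaveGame in the "NiceColors" slot, parsed by a shared lookup keyed on SaveGameID.
; Saving replaces or appends an entry, treating -1 components as keep-existing so wheel (H, S) and slider (V) save independently.
; Loading returns the stored HSV and whether it was found.
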(fn GetColorbyWheelandSliderRefs
  (params (ColorWheel :type WB%20Color%20Wheel%20Object%20Reference) (Slider :type WB%20Slider%20Color%20Wheel%20Value%20Object%20Reference))
  (bind _currentcolor (Variables|/Game/NiceColorWheel/Widgets/Master/WB_ColorWheel.WB_ColorWheel_C|GetCurrentColor ColorWheel))
  (bind _currentvalue (Variables|/Game/NiceColorWheel/Widgets/Master/WB_Slider_ColorWheelValue.WB_Slider_ColorWheelValue_C|GetCurrentValue Slider))
  (bind _returnvalue (* _currentcolor _currentvalue))
  (bind (_r _g _b) (Utilities|Struct|BreakLinearColor _returnvalue))
  (Utilities|IsValid ColorWheel
    (:Is%20Valid
      (Utilities|IsValid Slider
        (:Is%20Valid
          (return (Utilities|Struct|MakeLinearColor _r _g _b 1.0)))))))

(fn SaveHSVOfColorWheelorValueSlider
  (params (SaveGameRef :type BP%20Nice%20Color%20Wheel%20Save%20Game%20Object%20Reference%20%28by%20ref%29) (SaveGameID :type String) (HSV :type S%20HSV%20Structure%20%28by%20ref%29))
  (bind _v (Utilities|Struct|BreakS_HSV HSV))
  (bind (_h _s _v_2) (Utilities|Struct|BreakS_HSV HSV))
  (bind _h_2 (Utilities|Struct|BreakS_HSV HSV))
  (bind _s_2 (Utilities|Struct|BreakS_HSV HSV))
  ;[1 1 1] Check if and where this SaveGameID was saved
  (bind (_bfound _index _foundhsv) (CallFunction|FindFormattedColorWheelHandleIndex (Variables|/Game/NiceColorWheel/Blueprints/BP_NiceColorWheel_SaveGame.BP_NiceColorWheel_SaveGame_C|GetAllColorWheelAndHandleHSV_SaveData SaveGameRef) SaveGameID))
  (if _bfound
    ;[1 1 1] Replace current HSV values with new HSV values. However if a value is -1 it keeps the existing value. Usually the color wheel sets the H & S value while the slider sets the V value
    (bind _output_get (LocalVariables|SetSaveArrayCopy (Utilities|String|ParseIntoArray (Variables|/Game/NiceColorWheel/Blueprints/BP_NiceColorWheel_SaveGame.BP_NiceColorWheel_SaveGame_C|GetAllColorWheelAndHandleHSV_SaveData SaveGameRef) ";")))
    (Utilities|Array|SetArrayElem _output_get _index (Utilities|String|Append SaveGameID "=" (Utilities|String|ToString(Float) (select (== _h_2 -1.0) (.H (Utilities|Struct|BreakS_HSV _foundhsv)) _h_2)) "/" (Utilities|String|ToString(Float) (select (== _s_2 -1.0) (.S (Utilities|Struct|BreakS_HSV _foundhsv)) _s_2)) "/" (Utilities|String|ToString(Float) (select (== _v -1.0) (.V (Utilities|Struct|BreakS_HSV _foundhsv)) _v))) true)
    (Variables|/Game/NiceColorWheel/Blueprints/BP_NiceColorWheel_SaveGame.BP_NiceColorWheel_SaveGame_C|SetAllColorWheelAndHandleHSV_SaveData SaveGameRef (Utilities|String|JoinStringArray (LocalVariables|GetSaveArrayCopy) ";"))
    ;[1 1 1] Save to slot
    (SaveGame|SaveGametoSlot SaveGameRef "NiceColors")
    (else
      ;[1 1 1] SaveGameID was never saved - add new formatted entry containing HSV with the related SaveGameID
      (Variables|/Game/NiceColorWheel/Blueprints/BP_NiceColorWheel_SaveGame.BP_NiceColorWheel_SaveGame_C|SetAllColorWheelAndHandleHSV_SaveData SaveGameRef (Utilities|String|Append (Variables|/Game/NiceColorWheel/Blueprints/BP_NiceColorWheel_SaveGame.BP_NiceColorWheel_SaveGame_C|GetAllColorWheelAndHandleHSV_SaveData SaveGameRef) ";" (Utilities|String|Append SaveGameID "=" (Utilities|String|ToString(Float) _h) "/" (Utilities|String|ToString(Float) _s) "/" (Utilities|String|ToString(Float) _v_2))))
      ;[1 1 1] Save to slot
      (SaveGame|SaveGametoSlot SaveGameRef "NiceColors"))))

(fn LoadHSVOfColorWheelorValueSlider
  (params (SaveGameID :type String))
  (Utilities|FlowControl|Sequence
    (:then_0
      ;[1 1 1] Try to Load game from slot
      (bind _returnvalue (SaveGame|DoesSaveGameExist "NiceColors"))
      (if _returnvalue
        (bind _returnvalue_2 (SaveGame|LoadGamefromSlot "NiceColors"))
        (bind _asbp_nice_color_wheel_save_game (Utilities|Casting|CastToBP_NiceColorWheel_SaveGame _returnvalue_2))
        ;[1 1 1] Return HSV if entry was found for given SaveGameID
        (bind (_bfound _index _foundhsv) (CallFunction|FindFormattedColorWheelHandleIndex (Variables|/Game/NiceColorWheel/Blueprints/BP_NiceColorWheel_SaveGame.BP_NiceColorWheel_SaveGame_C|GetAllColorWheelAndHandleHSV_SaveData _asbp_nice_color_wheel_save_game) SaveGameID))
        (if _bfound
          (return true _foundhsv))))
    (:then_1
      ;[1 1 1] If there was no entry for the given SaveGameID return nothing
      (return false ""))))

(fn FindFormattedColorWheelHandleIndex
  (params (SaveDataString :type String) (SaveGameID :type String))
  ;[1 1 1] Search in formatted save game data string for the index and HSV value that is related to a certain SaveGameID
  (for (_array_element _array_index) (Utilities|String|ParseIntoArray SaveDataString ";")
    (if (Utilities|Enum|Equal(Enum) (.LeftS (Utilities|String|Split _array_element "=")) SaveGameID)
      (return true _array_index (Utilities|Struct|MakeS_HSV (Math|Conversions|ToFloat(Integer) (Utilities|Array|Get(acopy) (Utilities|String|ParseIntoArray (.RightS (Utilities|String|Split _array_element "=")) "/"))) (Math|Conversions|ToFloat(Integer) (Utilities|Array|Get(acopy) (Utilities|String|ParseIntoArray (.RightS (Utilities|String|Split _array_element "=")) "/") 1)) (Math|Conversions|ToFloat(Integer) (Utilities|Array|Get(acopy) (Utilities|String|ParseIntoArray (.RightS (Utilities|String|Split _array_element "=")) "/") 2))))))
  (return false -1 ""))