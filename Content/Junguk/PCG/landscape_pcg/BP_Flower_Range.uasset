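; BP_Flower_Range is an actor that selects and generates PCG graphs for flowers in a landscape.
; On BeginPlay, GetData matches the JS_RoomController's SubObject against PCGName in a flower data array, then assigns and generates that graph.
; ChangeFlower swaps in the graph from supplied flower data and regenerates.
; Both paths look up a PCGVolume and print debug names.
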(event Custom|ChangeFlower
  (params (FLowerData :type BP%20PCG%20Object%20Reference))
  (bind _pcg (Variables|Default|GetPCG))
  (Actor|GetActorOfClass "/Script/PCG.PCGVolume")
  (bind _output_get (Variables|data|SetFLowerData FLowerData))
  (Class|PCGComponent|SetGraph _pcg (Variables|/Game/KGw/UI/DataAsset/BP_PCG.BP_PCG_C|Getpcg _output_get))
  (Development|PrintString (Utilities|GetDisplayName _pcg))
  (PCG|Generate _pcg true))

(event Custom|GetData
  (bind _pcg (Variables|Default|GetPCG))
  (bind _asjs_room_controller (Utilities|Casting|CastToJS_RoomController (Game|GetPlayerController 0)))
  (Actor|GetActorOfClass "/Script/PCG.PCGVolume")
  (for _array_element (Variables|data|GetFLowerData_0)
    (if (== (Variables|/Game/KGw/UI/DataAsset/BP_PCG.BP_PCG_C|GetPCGName _array_element) (Variables|/Script/HttpTest.JS_RoomController|GetsubObject _asjs_room_controller))
      (Class|PCGComponent|SetGraph _pcg (Variables|/Game/KGw/UI/DataAsset/BP_PCG.BP_PCG_C|Getpcg _array_element))
      (Development|PrintString (Utilities|GetDisplayName (Variables|/Game/KGw/UI/DataAsset/BP_PCG.BP_PCG_C|Getpcg _array_element)) true true "(R=0.000000,G=0.660000,B=1.000000,A=1.000000)" 1e+01)
      (PCG|Generate _pcg true))))

(event EventBeginPlay
  (CallFunction|GetData))

(event Collision|EventActorBeginOverlap
  (params (OtherActor :type Actor%20Object%20Reference)))

(event EventTick
  (params (DeltaSeconds :type Float%20%28single-precision%29)))

(fn ConstructionScript)