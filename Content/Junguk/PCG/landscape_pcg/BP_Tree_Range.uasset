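; BP_Tree_Range drives procedural tree generation in the landscape by switching the graph on a PCG component.
; On BeginPlay it sets the main object, finds the TreeData0 entry whose PCGName matches it, then assigns that graph and generates.
; The ChangeTree event stores a supplied TreeData, swaps to its graph and regenerates at runtime.
; Both paths look up a PCGVolume and print debug names.
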(event Custom|ChangeTree
  (params (TreeData :type BP%20PCG%20Object%20Reference))
  (bind _pcg (Variables|Default|GetPCG))
  (Actor|GetActorOfClass "/Script/PCG.PCGVolume")
  (bind _output_get (Variables|Default|SetTreeData TreeData))
  (Class|PCGComponent|SetGraph _pcg (Variables|/Game/KGw/UI/DataAsset/BP_PCG.BP_PCG_C|Getpcg _output_get))
  (Development|PrintString (Utilities|GetDisplayName _pcg))
  (PCG|Generate _pcg true))

(event EventBeginPlay
  (bind _pcg (Variables|Default|GetPCG))
  (Class|CJSMainObjectActor|SetMainObject)
  (bind _returnvalue (Class|CJSMainObjectActor|GetMainObject))
  (Actor|GetActorOfClass "/Script/PCG.PCGVolume")
  (for _array_element (Variables|Default|GetTreeData_0)
    (if (== (Variables|/Game/KGw/UI/DataAsset/BP_PCG.BP_PCG_C|GetPCGName _array_element) _returnvalue)
      (Class|PCGComponent|SetGraph _pcg (Variables|/Game/KGw/UI/DataAsset/BP_PCG.BP_PCG_C|Getpcg _array_element))
      (Development|PrintString (Utilities|String|Append (Utilities|GetDisplayName (Variables|/Game/KGw/UI/DataAsset/BP_PCG.BP_PCG_C|Getpcg _array_element)) " : ah~~~~~~") true true "(R=0.000000,G=0.660000,B=1.000000,A=1.000000)" 1e+01)
      (PCG|Generate _pcg true))))

(fn ConstructionScript)