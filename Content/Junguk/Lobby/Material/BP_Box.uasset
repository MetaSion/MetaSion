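; BP_Box is a lobby material helper actor that publishes a box volume's placement to the PC_Box Material Parameter Collection.
; It writes Cube2's world location and world scale into the Location and Bounds vector parameters, so materials reading the collection can follow the box.
; The construction script and Tick both perform this write, covering editor changes and runtime movement.
; Cube_2's begin-overlap event casts to BP_Jk_Player but does nothing further.
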(event OnComponentBeginOverlap(Cube_2)
  (params (OverlappedComponent :type Primitive%20Component%20Object%20Reference) (OtherActor :type Actor%20Object%20Reference) (OtherComp :type Primitive%20Component%20Object%20Reference) (OtherBodyIndex :type Integer) (bFromSweep :type Boolean) (SweepResult :type Hit%20Result%20Structure%20%28by%20ref%29))
  (Utilities|Casting|CastToBP_Jk_Player OtherActor))

(event EventBeginPlay)

(event Collision|EventActorBeginOverlap
  (params (OtherActor :type Actor%20Object%20Reference)))

(event EventTick
  (params (DeltaSeconds :type Float%20%28single-precision%29))
  (bind _cube_2 (Variables|Default|GetCube_2))
  (Rendering|Material|SetVectorParameterValue "/Game/Junguk/Lobby/Material/PC_Box.PC_Box" "Location" (Math|Conversions|ToLinearColor(Vector) (Transformation|GetWorldLocation _cube_2)) :!class /Script/Engine.KismetMaterialLibrary)
  (Rendering|Material|SetVectorParameterValue "/Game/Junguk/Lobby/Material/PC_Box.PC_Box" "Bounds" (Math|Conversions|ToLinearColor(Vector) (Transformation|GetWorldScale _cube_2)) :!class /Script/Engine.KismetMaterialLibrary))

(fn ConstructionScript
  (bind _cube_2 (Variables|Default|GetCube_2))
  (Rendering|Material|SetVectorParameterValue "/Game/Junguk/Lobby/Material/PC_Box.PC_Box" "Location" (Math|Conversions|ToLinearColor(Vector) (Transformation|GetWorldLocation _cube_2)) :!class /Script/Engine.KismetMaterialLibrary)
  (Rendering|Material|SetVectorParameterValue "/Game/Junguk/Lobby/Material/PC_Box.PC_Box" "Bounds" (Math|Conversions|ToLinearColor(Vector) (Transformation|GetWorldScale _cube_2)) :!class /Script/Engine.KismetMaterialLibrary))