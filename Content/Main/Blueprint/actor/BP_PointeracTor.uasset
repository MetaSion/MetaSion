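; BP_PointeracTor is a pointer actor with a 3D text component, apparently meant to show Korean onboarding prompts about sharing moods, connecting players and AI-expressed emotion.
; Its graph holds timed text sequences using Delay, an arrow label and a call to hide login text.
; None of these chains is wired to an event, and BeginPlay, the construction script and NewFunction are empty, so the Blueprint currently runs no logic.
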(event EventBeginPlay)

(fn ConstructionScript)

(fn NewFunction)