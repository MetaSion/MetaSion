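; BP_Login_3DTextActor is a login intro actor that shows timed 3D text inviting the player to build a world with their emotion character and connect with others.
; On BeginPlay it hides the text, then uses a chain of delays to show it, swap between two hardcoded Korean lines, clear it and hide it again.
; When the sequence ends, it calls ReadyReqLoginData to signal readiness for the login data request.
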(event EventBeginPlay
  (Class|CJSText3DActor|HideLoginText3D)
  (Utilities|FlowControl|Delay 3.0)
  (Class|CJSText3DActor|ShowLoginText3D)
  (Variables|/Script/Text3D.Text3DComponent|SetText (Variables|Default|GetText3DComponent) "당신의 감정 캐릭터로 월드를 만들고")
  (Utilities|FlowControl|Delay 4.0)
  (Variables|/Script/Text3D.Text3DComponent|SetText (Variables|Default|GetText3DComponent) "다른 플레이어와 연결되어 보세요.")
  (Utilities|FlowControl|Delay 3.0)
  (Variables|/Script/Text3D.Text3DComponent|SetText (Variables|Default|GetText3DComponent) "")
  (Utilities|FlowControl|Delay 0.2)
  (Class|CJSText3DActor|HideLoginText3D)
  (Class|CJSText3DActor|ReadyReqLoginData))

(fn ConstructionScript)