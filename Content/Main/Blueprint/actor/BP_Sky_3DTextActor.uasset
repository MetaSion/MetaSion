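; Sky 3D text actor that shows a short Korean intro saying that answering three questions lets an AI express the player's emotions.
; On BeginPlay it steps Text3DComponent through two lines with timed delays, then calls HideLoginText3D.
; Disconnected chains hold an unused alternate sequence about sharing moods and connecting with other players, plus a text clear.
; The construction script and NewFunction are empty.
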(event EventBeginPlay
  (Variables|/Script/Text3D.Text3DComponent|SetText (Variables|Default|GetText3DComponent) "3가지 질문에 응답하면")
  (Utilities|FlowControl|Delay 3.0)
  (Variables|/Script/Text3D.Text3DComponent|SetText (Variables|Default|GetText3DComponent) "AI가 당신의 감정을 표현해 줄 거예요.")
  (Utilities|FlowControl|Delay 3.0)
  (Class|CJSText3DActor|HideLoginText3D))

(fn ConstructionScript)

(fn NewFunction)