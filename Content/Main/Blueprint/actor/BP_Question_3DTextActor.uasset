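; BP_Question_3DTextActor is a 3D text actor that displays Korean survey questions asking the player about mood, energy, and the season expressing their heart.
; Three custom events each set the Text3D component to one question, and only the first also calls ShowQuestionText3D.
; BeginPlay and construction are empty.
; Disconnected leftover nodes hold show, hide and delay calls, plus an unused prompt to connect with other players.
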(event Custom|ShowQuestion1
  (Class|CJSQuestion3DActor|ShowQuestionText3D)
  (Variables|/Script/Text3D.Text3DComponent|SetText (Variables|Default|GetText3DComponent) "당신의 기분을 알려주세요"))

(event Custom|Setquestion2
  (Variables|/Script/Text3D.Text3DComponent|SetText (Variables|Default|GetText3DComponent) "당신의 에너지를 알려주세요"))

(event Custom|SetQuestoin3
  (Variables|/Script/Text3D.Text3DComponent|SetText (Variables|Default|GetText3DComponent) "당신의 마음을 표현하는 계절을 알려주세요"))

(event EventBeginPlay)

(fn ConstructionScript)