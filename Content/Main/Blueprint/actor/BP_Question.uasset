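; BP_Question is an actor that shows numbered questions, held as three child actor components that all start hidden.
; GetIndexquestionNum rebuilds the QuestionNum array through ChangeQuestionNum, listing the components in reverse of their naming order.
; It then reveals the component at the given index and hides the one at the preceding index, with no bounds check.
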(event Custom|ChangeQuestionNum
  (Variables|Default|SetQuestionNum%20 (Utilities|Array|MakeArray (Variables|Default|GetChildActor2) (Variables|Default|GetChildActor1) (Variables|Default|GetChildActor))))

(event EventBeginPlay
  (Rendering|SetVisibility (Variables|Default|GetChildActor) false false)
  (Rendering|SetVisibility (Variables|Default|GetChildActor1) false false)
  (Rendering|SetVisibility (Variables|Default|GetChildActor2) false false))

(event Collision|EventActorBeginOverlap
  (params (OtherActor :type Actor%20Object%20Reference)))

(event EventTick
  (params (DeltaSeconds :type Float%20%28single-precision%29)))

(fn ConstructionScript)

(fn GetIndexquestionNum
  (params (Dimension%201 :type Integer))
  (CallFunction|ChangeQuestionNum)
  (Rendering|SetVisibility (Utilities|Array|Get(acopy) (Variables|Default|GetQuestionNum%20) Dimension%201) true false)
  (bind _result (Math|Integer|DecrementInt Dimension%201)
    (:%20%20
      (Rendering|SetVisibility (Utilities|Array|Get(acopy) (Variables|Default|GetQuestionNum%20) _result) false false))))