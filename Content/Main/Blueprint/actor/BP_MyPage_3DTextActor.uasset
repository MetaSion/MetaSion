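; My Page intro text actor that shows a short Korean message sequence promoting AI emotion analysis and recommendations.
; On BeginPlay it swaps the Text3D component's text through three lines with fixed Delay pauses, then hides itself and calls CallMyPageActor.
; ShowQuesionText3D is an empty event, and an unconnected branch about connecting with other players never runs.
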(event Custom|ShowQuesionText3D)

(event EventBeginPlay
  (Variables|/Script/Text3D.Text3DComponent|SetText (Variables|Default|GetText3DComponent) "당신을 위한")
  (Utilities|FlowControl|Delay 5.0)
  (Variables|/Script/Text3D.Text3DComponent|SetText (Variables|Default|GetText3DComponent) " AI 감정분석과  추천을 ")
  (Utilities|FlowControl|Delay 5.0)
  (Variables|/Script/Text3D.Text3DComponent|SetText (Variables|Default|GetText3DComponent) "확인해 보세요")
  (Utilities|FlowControl|Delay 5.0)
  (Rendering|SetActorHiddenInGame true)
  (Class|CJSMyPageText3DActor|CallMyPageActor))

(fn ConstructionScript)